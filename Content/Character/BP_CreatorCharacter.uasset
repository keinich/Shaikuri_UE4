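; BP_CreatorCharacter is a Character Blueprint, apparently for a creator view, whose input drives an orbit-style camera on a SpringArm.
; Turn and LookUp axes feed controller yaw and pitch.
; MoveForward shifts the spring arm vertically instead of walking, applying the move only while its height stays between zero and MaxSpringArmZ.
; ZoomIn adjusts the arm length by a scaled axis value, without any clamp.
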(event `InputAxis|MoveForward`
  (params (AxisValue :type "Float (single-precision)"))
  (bind _returnvalue (+ (`KismetMathLibrary.MakeVector` 0.0 0.0 AxisValue) (`SceneComponent.RelativeLocation` (`self.SpringArm`))))
  (bind _z (.z _returnvalue))
  ;[1 1 1] Camera Shift
  (if (and (>= _z 0.0) (< _z (`self.Max_SpringArm_Z`)))
    (`SceneComponent.K2_SetRelativeLocation` (`self.SpringArm`) _returnvalue false false)))

(event `InputAxis|Turn`
  (params (AxisValue :type "Float (single-precision)"))
  ;[1 1 1] Looking Around
  (`self.AddControllerYawInput` AxisValue))

(event `InputAxis|LookUp`
  (params (AxisValue :type "Float (single-precision)"))
  ;[1 1 1] Looking Around
  (`self.AddControllerPitchInput` AxisValue))

(event `InputAxis|ZoomIn`
  (params (AxisValue :type "Float (single-precision)"))
  (bind _springarm (`self.SpringArm`))
  ;[1 1 1] Zooming
  (set `SpringArmComponent.TargetArmLength` (+ (`SpringArmComponent.TargetArmLength` _springarm) (* AxisValue -20.0)) _springarm))

(fn `UserConstructionScript`)